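; Top-down player character with movement states, sprint stamina and a zoomable camera.
; Sprint, walk and aim inputs set flags and call ChangeMovementState, while a looping timer drains stamina during forward sprinting and otherwise regenerates it.
; Mouse wheel changes the spring-arm length within limits, either instantly or in timer-driven steps.
; Test keys play hip or ironsight fire montages and a camera shake, and Tick prints state, stamina and speed.
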(event `Key|SpaceBar`
  (params (Key :type "Key Structure"))
  (bind _mesh (`self.Mesh`))
  (:`Pressed`
    (if (`self.AimEnable`)
      (`|PlayMontage` _mesh "/Game/Blueprints/Character/Mannequin/NewAnim/NewFire_Rifle_Ironsights_Montage.NewFire_Rifle_Ironsights_Montage")
      (else
        (`|PlayMontage` _mesh "/Game/Blueprints/Character/Mannequin/NewAnim/NewFire_Rifle_Hip_Montage.NewFire_Rifle_Hip_Montage")))))

(event `Key|F`
  (params (Key :type "Key Structure"))
  (:`Pressed`
    (`self.CameraShakeEvent`)))

(event `InputAxis|MouseWheel`
  (params (AxisValue :type "Float (single-precision)"))
  (if (`self.SlideWithSmooth`)
    (`self.CameraSlideSmooth` AxisValue)
    (else
      (`self.CameraSlide` AxisValue))))

(event `InputAction|SprintMovement`
  (params (Key :type "Key Structure"))
  (:`Pressed`
    (set `self.SprintRunEnable` true)
    (`|ExecutionSequence`
      (:`then_0`
        (bind _returnvalue (`KismetSystemLibrary.K2_SetTimerDelegate` (delegate `Stamina Tick`) 1.0 true))
        (set `self.StaminaTimer` _returnvalue))
      (:`then_1`
        (`self.ChangeMovementState` :!label _label))))
  (:`Released`
    (set `self.SprintRunEnable` false)
    (goto _label)))

(event `Stamina Tick`
  (`self.StaminaFunc`))

(event `InputAction|WalkMovement`
  (params (Key :type "Key Structure"))
  (:`Pressed`
    (set `self.WalkEnable` true)
    (goto _label))
  (:`Released`
    (set `self.WalkEnable` false)
    (goto _label)))

(event `InputAction|AimMovement`
  (params (Key :type "Key Structure"))
  (:`Pressed`
    (set `self.AimEnable` true)
    (goto _label))
  (:`Released`
    (set `self.AimEnable` false)
    (goto _label)))

(event `self.ReceiveTick`
  (params (DeltaSeconds :type "Float (single-precision)"))
  (`KismetSystemLibrary.PrintString` (`KismetStringLibrary.Concat_StrStr` "Movement State: " (`|GetEnumeratorNameAsString` (`self.MovementState`))) true true (struct :`G` 0.66 :`B` 1.0 :`A` 1.0) 0.0)
  (`KismetSystemLibrary.PrintString` (`KismetStringLibrary.Concat_StrStr` "Stamina: " (`KismetStringLibrary.Conv_DoubleToString` (`self.Stamina`))) true true (struct :`G` 1.0 :`B` 0.061501 :`A` 1.0) 0.0)
  (`KismetSystemLibrary.PrintString` (`KismetStringLibrary.Concat_StrStr` "Speed: " (`KismetStringLibrary.Conv_DoubleToString` (`self.ResSpeed`))) true true (struct :`R` 1.0 :`B` 0.069327 :`A` 1.0) 0.0))

(fn `CameraShakeEvent`
  (`GameplayStatics.PlayWorldCameraShake` "/Game/Blueprints/Character/BP_CameraShake.BP_CameraShake_C" (`SceneComponent.K2_GetComponentLocation` (`self.TopDownCameraComponent`)) 0.0 30.0))

(fn `CameraSlide`
  (params (Value :type "Float (double-precision)"))
  (bind _cameraboom (`self.CameraBoom`))
  (bind _changedistanceheightcamera (`self.ChangeDistanceHeightCamera`))
  (bind _targetarmlength (`SpringArmComponent.TargetArmLength` _cameraboom))
  (bind _returnvalue (- _targetarmlength _changedistanceheightcamera))
  (bind _returnvalue_2 (+ _targetarmlength _changedistanceheightcamera))
  (if (!= Value 0.0)
    (if (< Value 0.0)
      (if (>= (`self.MaxCameraHeight`) _returnvalue_2)
        (set `SpringArmComponent.TargetArmLength` _returnvalue_2 _cameraboom))
      (elif (<= (`self.MinCameraHeight`) _returnvalue)
        (set `SpringArmComponent.TargetArmLength` _returnvalue _cameraboom)))))

(fn `CameraSlideSmooth`
  (params (Value :type "Float (double-precision)"))
  (bind _changedistanceheightcamera (`self.ChangeDistanceHeightCamera`))
  (bind _targetarmlength (`SpringArmComponent.TargetArmLength` (`self.CameraBoom`)))
  (if (`self.SlideDone`)
    (if (!= Value 0.0)
      (if (< Value 0.0)
        (if (>= (`self.MaxCameraHeight`) (+ _targetarmlength _changedistanceheightcamera))
          (set `self.SlideUp` true)
          (set `self.SlideDone` false :!label _label)
          (bind _returnvalue (`KismetSystemLibrary.K2_SetTimer` null "CameraSlideSmoothTick" (`self.TimerStep`) true))
          (set `self.SlideTimer` _returnvalue))
        (elif (<= (`self.MinCameraHeight`) (- _targetarmlength _changedistanceheightcamera))
          (set `self.SlideUp` false)
          (goto _label))))))

(fn `CameraSlideSmoothTick`
  (bind _changestepdistanceheightcamera (`self.ChangeStepDistanceHeightCamera`))
  (bind _cameraboom (`self.CameraBoom`))
  (bind _targetarmlength (`SpringArmComponent.TargetArmLength` _cameraboom))
  (bind _output_get (set `self.CurrentSlideDistance` (+ (`self.CurrentSlideDistance`) _changestepdistanceheightcamera)))
  (set `SpringArmComponent.TargetArmLength` (select `bool` (`self.SlideUp`) :`false` (- _targetarmlength _changestepdistanceheightcamera) :`true` (+ _targetarmlength _changestepdistanceheightcamera)) _cameraboom)
  (if (>= _output_get (`self.ChangeDistanceHeightCamera`))
    (set `self.CurrentSlideDistance` 0.0)
    (set `self.SlideDone` true)
    (`KismetSystemLibrary.K2_ClearAndInvalidateTimerHandle` (`self.SlideTimer`))))

(fn `StaminaFunc`
  (bind _returnvalue (`self.IsForvardMove`))
  (if (and _returnvalue (`self.SprintRunEnable`) (> (`self.Stamina`) 0.0))
    (bind _output_get (set `self.Stamina` (- (`self.Stamina`) 10.0)))
    (if (<= _output_get 0.0)
      (set `self.Stamina` 0.0)
      (set `self.SprintRunEnable` false)
      (`self.ChangeMovementState`))
    (else
      (set `self.SprintRunEnable` false)
      (`self.ChangeMovementState`)
      (bind _output_get_2 (set `self.Stamina` (+ (`self.Stamina`) 5.0)))
      (if (>= _output_get_2 100.0)
        (`KismetSystemLibrary.K2_ClearAndInvalidateTimerHandle` (`self.StaminaTimer`))
        (set `self.Stamina` 100.0)))))

(fn `UserConstructionScript`
  (bind _cameraboom (`self.CameraBoom`))
  (set `SpringArmComponent.TargetArmLength` (`self.DefaultCameraHieght`) _cameraboom)
  (`SceneComponent.K2_SetRelativeRotation` _cameraboom (`self.CameraRotation`) false false)
  (set `SpringArmComponent.bEnableCameraLag` (`self.Flow`) _cameraboom)
  (set `SpringArmComponent.CameraLagSpeed` (`self.Smooth`) _cameraboom))